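; LightPad is a floor-pad actor that toggles its On state, and that of every pad in its Pads array, when FirstPersonCharacter overlaps its Box.
; The linked-pad loop also runs a DoOnce that damages the character and plays an explosion sound and particle, resetting after a short delay.
; Tick swaps the Cube material each frame to show the current On state.
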(event `self.Box.OnComponentBeginOverlap`
  (params (OverlappedComponent :type "PrimitiveComponent Object Reference") (OtherActor :type "Actor Object Reference") (OtherComp :type "PrimitiveComponent Object Reference") (OtherBodyIndex :type Integer) (bFromSweep :type Boolean) (SweepResult :type "HitResult Structure (by ref)"))
  (bind _returnvalue (`self.K2_GetActorLocation`))
  (if (== (`GameplayStatics.GetObjectClass` OtherActor) "/Game/FirstPersonBP/Blueprints/FirstPersonCharacter.FirstPersonCharacter_C")
    (if (`self.on`)
      (set `self.on` false)
      (else
        (set `self.on` true)))
    (for _array_element (`self.Pads`)
      (if (`/Game/Blueprints/LightPad.on` _array_element)
        (set `/Game/Blueprints/LightPad.on` false _array_element)
        (else
          (set `/Game/Blueprints/LightPad.on` true _array_element)))
      (`/Engine/EditorBlueprintResources/StandardMacros.DoOnce` false :!label _label
        (:`Completed`
          (`GameplayStatics.ApplyDamage` OtherActor (`self.Base Damage`))
          (`GameplayStatics.PlaySoundAtLocation` "/Game/StarterContent/Audio/Explosion01.Explosion01" _returnvalue (struct) 1.0 1.0 0.0 null null null)
          (`GameplayStatics.SpawnEmitterAtLocation` "/Game/StarterContent/Particles/P_Explosion.P_Explosion" _returnvalue)
          (`KismetSystemLibrary.Delay` 1.0)
          (goto _label :!via `Reset`))))))

(event `self.ReceiveTick`
  (params (DeltaSeconds :type "Float (single-precision)"))
  (bind _cube (`self.Cube`))
  (if (`self.on`)
    (`PrimitiveComponent.SetMaterial` _cube 0 "/Game/Materials/OnTrue.OnTrue")
    (else
      (`PrimitiveComponent.SetMaterial` _cube 0 "/Game/Materials/OnFalse.OnFalse"))))

(fn `UserConstructionScript`)