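; Elevator door actor that reacts to the power box state and marks the win point for the player.
; Every Tick it looks up all Powerbox actors and, if the first has PowerOff set, snaps both door panels to fixed relative positions without interpolation.
; A separate Box overlap prints "WIN" when the player's capsule enters, independent of the power state.
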(event `self.ReceiveTick`
  (params (DeltaSeconds :type "Float (single-precision)"))
  (bind _outactors (`GameplayStatics.GetAllActorsOfClass` "/Game/Blueprints/Powerbox.Powerbox_C"))
  (if (`/Game/Blueprints/Powerbox.PowerOff` (`|GetArrayItem` _outactors))
    (`|ExecutionSequence`
      (:`then_0`
        (`SceneComponent.K2_SetRelativeLocation` (`self.RightDoor`) (100.0 -450.0 0.0) false false))
      (:`then_1`
        (`SceneComponent.K2_SetRelativeLocation` (`self.LeftDoor`) (-200.0 -450.0 0.0) false false)))))

(event `self.Box.OnComponentBeginOverlap`
  (params (OverlappedComponent :type "PrimitiveComponent Object Reference") (OtherActor :type "Actor Object Reference") (OtherComp :type "PrimitiveComponent Object Reference") (OtherBodyIndex :type Integer) (bFromSweep :type Boolean) (SweepResult :type "HitResult Structure (by ref)"))
  (if (== OtherComp (`Character.CapsuleComponent` (`GameplayStatics.GetPlayerCharacter` 0)))
    (`KismetSystemLibrary.PrintString` "WIN")))

(fn `UserConstructionScript`)