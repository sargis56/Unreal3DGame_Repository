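; Powerbox actor that lets the player switch off the power once they have obtained the required tool.
; When the player's capsule enters its box trigger, it finds the first Wrench actor in the level and checks its WrenchObtained flag.
; If obtained, it sets PowerOff; otherwise it leaves it unchanged, showing a timed message on the first-person character either way.
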(event `self.Powerbox Box.OnComponentBeginOverlap`
  (params (OverlappedComponent :type "PrimitiveComponent Object Reference") (OtherActor :type "Actor Object Reference") (OtherComp :type "PrimitiveComponent Object Reference") (OtherBodyIndex :type Integer) (bFromSweep :type Boolean) (SweepResult :type "HitResult Structure (by ref)"))
  (bind _returnvalue (`GameplayStatics.GetPlayerCharacter` 0))
  (if (== OtherComp (`Character.CapsuleComponent` _returnvalue))
    (bind _outactors (`GameplayStatics.GetAllActorsOfClass` "/Game/Blueprints/Wrench.Wrench_C"))
    (if (`/Game/Blueprints/Wrench.WrenchObtained` (`|GetArrayItem` _outactors))
      (set `self.PowerOff` true)
      (bind _asfirst_person_character (cast `/Game/FirstPersonBP/Blueprints/FirstPersonCharacter` _returnvalue))
      (`/Game/FirstPersonBP/Blueprints/FirstPersonCharacter.DisplayMessage` _asfirst_person_character "Power Is Now Off" 3.0)
      (else
        (bind _asfirst_person_character_2 (cast `/Game/FirstPersonBP/Blueprints/FirstPersonCharacter` _returnvalue))
        (`/Game/FirstPersonBP/Blueprints/FirstPersonCharacter.DisplayMessage` _asfirst_person_character_2 "Comeback With The Screwdriller To Turn Off The Power" 3.0)))))

(fn `UserConstructionScript`)