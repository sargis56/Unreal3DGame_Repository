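; Elevator door Blueprint that opens and closes a pair of sliding doors based on the On state of linked light pads.
; Every Tick it loops through the Pad array and sets both doors' relative locations to open or closed, snapping without interpolation or sweep.
; Each pad overwrites the previous result, so the last pad in the array decides the final door position.
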(event `self.ReceiveTick`
  (params (DeltaSeconds :type "Float (single-precision)"))
  (for _array_element (`self.Pad`)
    (if (`/Game/Blueprints/LightPad.on` (`|GetArrayItem` (`|MakeArray` _array_element)))
      (`|ExecutionSequence`
        (:`then_0`
          (`SceneComponent.K2_SetRelativeLocation` (`self.RightDoor`) (100.0 -450.0 0.0) false false))
        (:`then_1`
          (`SceneComponent.K2_SetRelativeLocation` (`self.LeftDoor`) (-200.0 -450.0 0.0) false false)))
      (else
        (`|ExecutionSequence`
          (:`then_0`
            (`SceneComponent.K2_SetRelativeLocation` (`self.RightDoor`) (0.0 -450.0 0.0) false false))
          (:`then_1`
            (`SceneComponent.K2_SetRelativeLocation` (`self.LeftDoor`) (-100.0 -450.0 0.0) false false)))))))

(fn `UserConstructionScript`)