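; Skeeball arcade machine actor that scores thrown balls, tracks a seven-ball round and shows points and throws left on text components.
; Overlap triggers match Skeeball actors' Box components, destroy the ball and spawn another at the machine's Box.
; Scoring holes add points and count a throw, OutOfBoard counts only the throw, and Room just respawns.
; Tick prints WIN at exactly 200 points, resets finished rounds and refreshes the text.
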(event `self.ReceiveTick`
  (params (DeltaSeconds :type "Float (single-precision)"))
  (`|ExecutionSequence`
    (:`then_0`
      (if (== (`self.Points`) 200)
        (`KismetSystemLibrary.PrintString` "WIN")))
    (:`then_1`
      (if (== (`self.BallsThrown`) 7)
        (set `self.BallsThrown` 0)
        (set `self.Points` 0)))
    (:`then_2`
      (`TextRenderComponent.K2_SetText` (`self.PointsText`) (`KismetTextLibrary.Conv_IntToText` (`self.Points`)))
      (`TextRenderComponent.K2_SetText` (`self.ThrowText1`) (`KismetTextLibrary.Conv_IntToText` (- 7 (`self.BallsThrown`)))))))

(event `self.ReceiveBeginPlay`
  (`|SpawnActorFromClass` "/Game/Blueprints/Skeeball.Skeeball_C" (`KismetMathLibrary.Conv_VectorToTransform` (`SceneComponent.K2_GetComponentLocation` (`self.Box`))) "Undefined" "OverrideRootScale" null null))

(event `self.10points.OnComponentBeginOverlap`
  (params (OverlappedComponent :type "PrimitiveComponent Object Reference") (OtherActor :type "Actor Object Reference") (OtherComp :type "PrimitiveComponent Object Reference") (OtherBodyIndex :type Integer) (bFromSweep :type Boolean) (SweepResult :type "HitResult Structure (by ref)"))
  (bind _outactors (`GameplayStatics.GetAllActorsOfClass` "/Game/Blueprints/Skeeball.Skeeball_C"))
  (for _array_element _outactors
    (if (== OtherComp (`/Game/Blueprints/Skeeball.Box` _array_element))
      (`self.K2_DestroyActor` OtherActor)
      (`|SpawnActorFromClass` "/Game/Blueprints/Skeeball.Skeeball_C" (`KismetMathLibrary.Conv_VectorToTransform` (`SceneComponent.K2_GetComponentLocation` (`self.Box`))) "Undefined" "OverrideRootScale" null null)
      (set `self.Points` (+ (`self.Points`) 10))
      (bind _result (`/Engine/EditorBlueprintResources/StandardMacros.IncrementInt` (`self.BallsThrown`))
        (:`  `
          (set `self.BallsThrown` _result))))))

(event `self.Room.OnComponentBeginOverlap`
  (params (OverlappedComponent :type "PrimitiveComponent Object Reference") (OtherActor :type "Actor Object Reference") (OtherComp :type "PrimitiveComponent Object Reference") (OtherBodyIndex :type Integer) (bFromSweep :type Boolean) (SweepResult :type "HitResult Structure (by ref)"))
  (bind _outactors (`GameplayStatics.GetAllActorsOfClass` "/Game/Blueprints/Skeeball.Skeeball_C"))
  (for _array_element _outactors
    (if (== OtherComp (`/Game/Blueprints/Skeeball.Box` _array_element))
      (`self.K2_DestroyActor` OtherActor)
      (`|SpawnActorFromClass` "/Game/Blueprints/Skeeball.Skeeball_C" (`KismetMathLibrary.Conv_VectorToTransform` (`SceneComponent.K2_GetComponentLocation` (`self.Box`))) "Undefined" "OverrideRootScale" null null))))

(event `self.OutOfBoard.OnComponentBeginOverlap`
  (params (OverlappedComponent :type "PrimitiveComponent Object Reference") (OtherActor :type "Actor Object Reference") (OtherComp :type "PrimitiveComponent Object Reference") (OtherBodyIndex :type Integer) (bFromSweep :type Boolean) (SweepResult :type "HitResult Structure (by ref)"))
  (bind _outactors (`GameplayStatics.GetAllActorsOfClass` "/Game/Blueprints/Skeeball.Skeeball_C"))
  (for _array_element _outactors
    (if (== OtherComp (`/Game/Blueprints/Skeeball.Box` _array_element))
      (`self.K2_DestroyActor` OtherActor)
      (`|SpawnActorFromClass` "/Game/Blueprints/Skeeball.Skeeball_C" (`KismetMathLibrary.Conv_VectorToTransform` (`SceneComponent.K2_GetComponentLocation` (`self.Box`))) "Undefined" "OverrideRootScale" null null)
      (bind _result (`/Engine/EditorBlueprintResources/StandardMacros.IncrementInt` (`self.BallsThrown`))
        (:`  `
          (set `self.BallsThrown` _result))))))

(event `self.100points.OnComponentBeginOverlap`
  (params (OverlappedComponent :type "PrimitiveComponent Object Reference") (OtherActor :type "Actor Object Reference") (OtherComp :type "PrimitiveComponent Object Reference") (OtherBodyIndex :type Integer) (bFromSweep :type Boolean) (SweepResult :type "HitResult Structure (by ref)"))
  (bind _outactors (`GameplayStatics.GetAllActorsOfClass` "/Game/Blueprints/Skeeball.Skeeball_C"))
  (for _array_element _outactors
    (if (== OtherComp (`/Game/Blueprints/Skeeball.Box` _array_element))
      (`self.K2_DestroyActor` OtherActor)
      (`|SpawnActorFromClass` "/Game/Blueprints/Skeeball.Skeeball_C" (`KismetMathLibrary.Conv_VectorToTransform` (`SceneComponent.K2_GetComponentLocation` (`self.Box`))) "Undefined" "OverrideRootScale" null null)
      (set `self.Points` (+ (`self.Points`) 100))
      (bind _result (`/Engine/EditorBlueprintResources/StandardMacros.IncrementInt` (`self.BallsThrown`))
        (:`  `
          (set `self.BallsThrown` _result))))))

(event `self.50points.OnComponentBeginOverlap`
  (params (OverlappedComponent :type "PrimitiveComponent Object Reference") (OtherActor :type "Actor Object Reference") (OtherComp :type "PrimitiveComponent Object Reference") (OtherBodyIndex :type Integer) (bFromSweep :type Boolean) (SweepResult :type "HitResult Structure (by ref)"))
  (bind _outactors (`GameplayStatics.GetAllActorsOfClass` "/Game/Blueprints/Skeeball.Skeeball_C"))
  (for _array_element _outactors
    (if (== OtherComp (`/Game/Blueprints/Skeeball.Box` _array_element))
      (`self.K2_DestroyActor` OtherActor)
      (`|SpawnActorFromClass` "/Game/Blueprints/Skeeball.Skeeball_C" (`KismetMathLibrary.Conv_VectorToTransform` (`SceneComponent.K2_GetComponentLocation` (`self.Box`))) "Undefined" "OverrideRootScale" null null)
      (set `self.Points` (+ (`self.Points`) 50))
      (bind _result (`/Engine/EditorBlueprintResources/StandardMacros.IncrementInt` (`self.BallsThrown`))
        (:`  `
          (set `self.BallsThrown` _result))))))

(event `self.40points.OnComponentBeginOverlap`
  (params (OverlappedComponent :type "PrimitiveComponent Object Reference") (OtherActor :type "Actor Object Reference") (OtherComp :type "PrimitiveComponent Object Reference") (OtherBodyIndex :type Integer) (bFromSweep :type Boolean) (SweepResult :type "HitResult Structure (by ref)"))
  (bind _outactors (`GameplayStatics.GetAllActorsOfClass` "/Game/Blueprints/Skeeball.Skeeball_C"))
  (for _array_element _outactors
    (if (== OtherComp (`/Game/Blueprints/Skeeball.Box` _array_element))
      (`self.K2_DestroyActor` OtherActor)
      (`|SpawnActorFromClass` "/Game/Blueprints/Skeeball.Skeeball_C" (`KismetMathLibrary.Conv_VectorToTransform` (`SceneComponent.K2_GetComponentLocation` (`self.Box`))) "Undefined" "OverrideRootScale" null null)
      (set `self.Points` (+ (`self.Points`) 40))
      (bind _result (`/Engine/EditorBlueprintResources/StandardMacros.IncrementInt` (`self.BallsThrown`))
        (:`  `
          (set `self.BallsThrown` _result))))))

(event `self.30points.OnComponentBeginOverlap`
  (params (OverlappedComponent :type "PrimitiveComponent Object Reference") (OtherActor :type "Actor Object Reference") (OtherComp :type "PrimitiveComponent Object Reference") (OtherBodyIndex :type Integer) (bFromSweep :type Boolean) (SweepResult :type "HitResult Structure (by ref)"))
  (bind _outactors (`GameplayStatics.GetAllActorsOfClass` "/Game/Blueprints/Skeeball.Skeeball_C"))
  (for _array_element _outactors
    (if (== OtherComp (`/Game/Blueprints/Skeeball.Box` _array_element))
      (`self.K2_DestroyActor` OtherActor)
      (`|SpawnActorFromClass` "/Game/Blueprints/Skeeball.Skeeball_C" (`KismetMathLibrary.Conv_VectorToTransform` (`SceneComponent.K2_GetComponentLocation` (`self.Box`))) "Undefined" "OverrideRootScale" null null)
      (set `self.Points` (+ (`self.Points`) 30))
      (bind _result (`/Engine/EditorBlueprintResources/StandardMacros.IncrementInt` (`self.BallsThrown`))
        (:`  `
          (set `self.BallsThrown` _result))))))

(fn `UserConstructionScript`)